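; Fishing boat hazard that kills the player as bycatch when its box overlaps them, showing a death screen.
; On spawn it registers with the Spawner, aims ahead of the player's movement with random yaw spread, and spawns fish linked to itself.
; While the player lives it drives straight forward, faster when distant.
; When too far away it decrements the Spawner count and destroys itself.
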(event OnComponentBeginOverlap(Box)
  (params (OverlappedComponent :type Primitive%20Component%20Object%20Reference) (OtherActor :type Actor%20Object%20Reference) (OtherComp :type Primitive%20Component%20Object%20Reference) (OtherBodyIndex :type Integer) (bFromSweep :type Boolean) (SweepResult :type Hit%20Result%20Structure%20%28by%20ref%29))
  (if (== OtherActor (Game|GetPlayerCharacter 0))
    (bind _asbp_third_person_character (Utilities|Casting|CastToBP_ThirdPersonCharacter (Game|GetPlayerCharacter 0)))
    (Default|Die _asbp_third_person_character)
    (bind _returnvalue (UserInterface|CreateWidget "/Game/mainMenu/BycatchDeathScreen.BycatchDeathScreen_C"))
    (UserInterface|Viewport|AddtoViewport _returnvalue 0)
    (Default|PlayAnimation _returnvalue)))

(event Custom|spawned
  (bind _returnvalue (Game|GetPlayerCharacter 0))
  (bind _rootcomponent (Variables|/Script/Engine.Actor|GetRootComponent _returnvalue))
  (bind _returnvalue_2 (Transformation|GetWorldLocation _rootcomponent))
  (Variables|Default|Setoffset (+ (Transformation|GetDistanceTo (Game|GetPlayerCharacter 0)) 2e+03))
  (bind _outactors (Actor|GetAllActorsOfClass "/Game/spawner.spawner_C"))
  (Default|Add1 (Utilities|Array|Get(acopy) _outactors))
  (bind _asbp_third_person_character (Utilities|Casting|CastToBP_ThirdPersonCharacter (Game|GetPlayerCharacter 0)))
  (Transformation|SetActorRotation (Math|Rotator|MakeRotator 0.0 0.0 (+ (.yaw (Math|Rotator|FindLookatRotation (Transformation|GetWorldLocation (Variables|Collision|GetCapsuleComponent)) (Math|Vector|MakeVector (+ (* (Variables|/Game/BP_ThirdPersonCharacter.BP_ThirdPersonCharacter_C|GetxMovement _asbp_third_person_character) (Variables|Default|Getoffset)) (.x _returnvalue_2)) (+ (.y _returnvalue_2) (* (Variables|/Game/BP_ThirdPersonCharacter.BP_ThirdPersonCharacter_C|GetyMovement _asbp_third_person_character) (Variables|Default|Getoffset))) (.z _returnvalue_2)))) (Math|Random|RandomFloatinRange -15.0 15.0))))
  (for _index (range 0 2)
    (bind _returnvalue_3 (Game|SpawnActorfromClass "/Game/fish.fish_C" (Transformation|GetActorTransform) "Undefined" 0 0))
    (Utilities|IsValid _returnvalue_3
      (:Is%20Valid
        (Pawn|SpawnDefaultController _returnvalue_3)
        (Default|BoatSpawn _returnvalue_3 self)
        (Audio|SpawnSoundAttached "/Game/soundEffect/mixkit-tank-engine-working-2753.mixkit-tank-engine-working-2753" (Variables|Collision|GetCapsuleComponent) "None" "0, 0, 0" "0, 0, 0" "KeepRelativeOffset" false 1.0 1.0 0.0 0 0)))))

(event Custom|kill
  (bind _outactors (Actor|GetAllActorsOfClass "/Game/spawner.spawner_C"))
  (Default|Minus1 (Utilities|Array|Get(acopy) _outactors))
  (Actor|DestroyActor (Pawn|GetController))
  (Actor|DestroyActor))

(event EventTick
  (params (DeltaSeconds :type Float%20%28single-precision%29))
  (bind _returnvalue (Game|GetPlayerCharacter 0))
  (bind _charactermovement (Variables|Character|GetCharacterMovement))
  (bind _returnvalue_2 (Transformation|GetDistanceTo _returnvalue))
  (if (> _returnvalue_2 2e+03)
    (Variables|/Script/Engine.CharacterMovementComponent|SetMaxWalkSpeed _charactermovement 2e+03)
    (else
      (Variables|/Script/Engine.CharacterMovementComponent|SetMaxWalkSpeed _charactermovement 8.5e+02)))
  (bind _asbp_third_person_character (Utilities|Casting|CastToBP_ThirdPersonCharacter (Game|GetPlayerCharacter 0)))
  (if (Variables|/Game/BP_ThirdPersonCharacter.BP_ThirdPersonCharacter_C|Getalive _asbp_third_person_character)
    (Pawn|Input|AddMovementInput (Transformation|GetActorForwardVector) 1.0 false)
    (if (> _returnvalue_2 6e+03)
      (CallFunction|Kill))))

(fn ConstructionScript)