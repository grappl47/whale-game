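; Whale hunter enemy character that relentlessly chases the player and kills them on close contact.
; Each tick, while the player is alive, it turns toward them and moves forward, triggering a one-time Attack that calls Die and shows an animated death screen.
; It teleports to a randomized offset around the player on spawn and whenever left too far behind, and carries an attached hum sound.
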(event Custom|Attack
  (if (not (Variables|Default|Getattacked))
    (bind _asbp_third_person_character (Utilities|Casting|CastToBP_ThirdPersonCharacter (Game|GetPlayerCharacter 0)))
    (Default|Die _asbp_third_person_character)
    (bind _returnvalue (UserInterface|CreateWidget "/Game/mainMenu/HunterDeathScreen.HunterDeathScreen_C" (Game|GetPlayerController 0)))
    (UserInterface|Viewport|AddtoViewport _returnvalue 0)
    (Default|PlayAnimation _returnvalue)))

(event Custom|teleport
  (bind _returnvalue (Game|GetPlayerCharacter 0))
  (bind _returnvalue_2 (Transformation|GetActorLocation _returnvalue))
  (if (== (Math|Random|RandomIntegerinRange 0 1) 0)
    (Variables|Default|SetminY 1.5e+03)
    (Variables|Default|SetmaxX 3e+03)
    (else
      (Variables|Default|SetminY -3e+03)
      (Variables|Default|SetmaxX -1.5e+03)))
  (if (== (Math|Random|RandomIntegerinRange 0 1) 0)
    (Variables|Default|SetminY 1.5e+03)
    (Variables|Default|SetmaxY 3e+03)
    (else
      (Variables|Default|SetminY -3e+03)
      (Variables|Default|SetmaxY -1.5e+03)))
  (Transformation|SetWorldLocation (Variables|Collision|GetCapsuleComponent) (Math|Vector|MakeVector (+ (.x _returnvalue_2) (Math|Random|RandomFloatinRange (Variables|Default|GetminX) (Variables|Default|GetmaxX))) (+ (.y _returnvalue_2) (Math|Random|RandomFloatinRange (Variables|Default|GetminY) (Variables|Default|GetmaxY))) 2e+02) false true)
  (Development|PrintString "teleported!!!!!!!!!!!!!!!!!!!!!!!!!!!!!!!!!!!!!!!!!!!!!!!!!!!!!!!!!!!!"))

(event EventBeginPlay
  (CallFunction|Teleport)
  (bind _returnvalue (Audio|SpawnSoundAttached "/Game/soundEffect/mixkit-game-ship-hum-3079.mixkit-game-ship-hum-3079" (Variables|Collision|GetCapsuleComponent) "None" "0, 0, 0" "0, 0, 0" "KeepRelativeOffset" false 1.0 1.0 0.0 0 0))
  (Audio|Components|Audio|AdjustVolume _returnvalue 0.0 2.0 "Linear" :!class /Script/Engine.AudioComponent))

(event EventTick
  (params (DeltaSeconds :type Float%20%28single-precision%29))
  (bind _returnvalue (Game|Player|GetPlayerPawn 0))
  (bind _returnvalue_2 (Transformation|GetDistanceTo _returnvalue))
  (bind _asbp_third_person_character (Utilities|Casting|CastToBP_ThirdPersonCharacter (Game|GetPlayerCharacter 0)))
  (if (Variables|/Game/BP_ThirdPersonCharacter.BP_ThirdPersonCharacter_C|Getalive _asbp_third_person_character)
    (Transformation|SetActorRotation (Math|Rotator|MakeRotator 0.0 0.0 (.yaw (Math|Rotator|FindLookatRotation (Transformation|GetWorldLocation (Variables|Collision|GetCapsuleComponent)) (Transformation|GetWorldLocation (Variables|/Script/Engine.Character|GetCapsuleComponent (Game|GetPlayerCharacter 0)))))))
    (Pawn|Input|AddMovementInput (Math|Vector|GetForwardVector (Variables|Collision|GetCapsuleComponent)) 1.0 false)
    (if (< _returnvalue_2 3e+02)
      (CallFunction|Attack)
      (Variables|Default|Setattacked true)
      (elif (> _returnvalue_2 6e+03)
        (CallFunction|Teleport)))))

(fn ConstructionScript)